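; BP_TilePuzleManager runs a tile puzzle, tracking progress across the BP_Tile actors that share its Id.
; On BeginPlay it gathers those tiles, sets itself as their Parent and uses their number as the required count.
; AddCount increments progress and calls Win, currently an empty stub, on reaching that total.
; CheckOverlaps calls ResetCount when no overlap is validated, clearing progress, raising disabled tiles and resetting colors unless already won.
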(event EventBeginPlay
  (bind _outactors (Actor|GetAllActorsOfClass "/Game/Matias/Puzles/TilesPuzle/BP_Tile.BP_Tile_C"))
  (for _array_element _outactors
    (if (== (Variables|Default|GetId) (Variables|/Game/Matias/Puzles/TilesPuzle/BP_Tile.BP_Tile_C|GetId _array_element))
      (Utilities|Array|Add (Variables|Default|GetTiles) _array_element)
      (Variables|/Game/Matias/Puzles/TilesPuzle/BP_Tile.BP_Tile_C|SetParent _array_element self)))
  (Variables|Default|SetTotalRequired (Utilities|Array|Length (Variables|Default|GetTiles))))

(fn ConstructionScript)

(fn AddCount
  (bind _result (Math|Integer|IncrementInt (Variables|Default|GetCurrentCount))
    (:%20%20
      (bind _output_get (Variables|Default|SetWinCondition (== _result (Variables|Default|GetTotalRequired))))
      (if _output_get
        (CallFunction|Win)))))

(fn ResetCount
  (if (not (Variables|Default|GetWinCondition))
    (Variables|Default|SetCurrentCount 0)
    (for _array_element (Variables|Default|GetTiles)
      (if (Variables|/Game/Matias/Puzles/TilesPuzle/BP_Tile.BP_Tile_C|Getenable _array_element)
        _
        (else
          (Default|UpPlatform _array_element)))
      (Default|ResetColor _array_element))))

(fn CheckOverlaps
  (bind _array_element (Utilities|Array|ForEachLoopwithBreak (Variables|Default|GetTiles) :!label _label)
    (:LoopBody
      (if (Variables|/Game/Matias/Puzles/TilesPuzle/BP_Tile.BP_Tile_C|GetisOverlap _array_element)
        (LocalVariables|SetValidate (Variables|/Game/Matias/Puzles/TilesPuzle/BP_Tile.BP_Tile_C|GetisOverlap _array_element))
        (goto _label Break)))
    (:Completed
      (if (not (LocalVariables|GetValidate))
        (CallFunction|ResetCount)))))

(fn Win)
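; Pressure tile for a step-on puzzle, reacting to the top-down player character until its Parent's win condition is met.
; Stepping on it lowers the cube via a timeline and turns it green, adding to the Parent's count.
; Stepping on it again before a reset turns it red and resets that count after a short delay.
; Leaving triggers the Parent's overlap check; separate events raise the tile and restore its color.
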(event OnComponentBeginOverlap(Box)
  (params (OverlappedComponent :type Primitive%20Component%20Object%20Reference) (OtherActor :type Actor%20Object%20Reference) (OtherComp :type Primitive%20Component%20Object%20Reference) (OtherBodyIndex :type Integer) (bFromSweep :type Boolean) (SweepResult :type Hit%20Result%20Structure%20%28by%20ref%29))
  (bind _parent (Variables|Default|GetParent))
  (bind _cube (Variables|Default|GetCube))
  (bind _parent_2 (Variables|Default|GetParent))
  (Utilities|Casting|CastToBP_Grupo5_TopDownCharacter OtherActor)
  (Utilities|IsValid _parent_2
    (:Is%20Valid
      (if (not (Variables|/Game/Matias/Puzles/TilesPuzle/BP_TilePuzleManager.BP_TilePuzleManager_C|GetWinCondition _parent_2))
        (Variables|Default|SetisOverlap true)
        (CallFunction|DownPlatform)
        (if (Variables|Default|Getenable)
          (Variables|Default|Setenable false)
          (Rendering|Material|SetMaterial _cube 0 "/Game/Matias/Puzles/Materials/MI_GreenInstance.MI_GreenInstance")
          (Default|AddCount _parent)
          (else
            (Rendering|Material|SetMaterial _cube 0 "/Game/Matias/Puzles/Materials/MI_RedInstance.MI_RedInstance")
            (Utilities|FlowControl|Delay 0.4)
            (Default|ResetCount _parent)))))))

(event OnComponentEndOverlap(Box)
  (params (OverlappedComponent :type Primitive%20Component%20Object%20Reference) (OtherActor :type Actor%20Object%20Reference) (OtherComp :type Primitive%20Component%20Object%20Reference) (OtherBodyIndex :type Integer))
  (bind _parent (Variables|Default|GetParent))
  (Utilities|Casting|CastToBP_Grupo5_TopDownCharacter OtherActor)
  (Utilities|IsValid _parent
    (:Is%20Valid
      (if (not (Variables|/Game/Matias/Puzles/TilesPuzle/BP_TilePuzleManager.BP_TilePuzleManager_C|GetWinCondition _parent))
        (Variables|Default|SetisOverlap false)
        (Default|CheckOverlaps _parent)))))

(event Custom|ResetColor
  (Rendering|Material|SetMaterial (Variables|Default|GetCube) 0 "/Game/Matias/Puzles/Materials/MAT_MasterColor.MAT_MasterColor")
  (Variables|Default|Setenable true))

(event Custom|UpPlatform
  (bind _location (Variables|Default|GetLocation))
  (bind _newtrack_0 (Timeline|Move ReverseFromEnd)
    (:Update
      (Transformation|SetWorldLocation (Variables|Default|GetCube) (Math|Vector|MakeVector (.x _location) (.y _location) (+ (.z _location) _newtrack_0)) false false))))

(event Custom|DownPlatform
  (bind _location (Variables|Default|GetLocation))
  (bind _newtrack_0 (Timeline|Move PlayFromStart)
    (:Update
      (Transformation|SetWorldLocation (Variables|Default|GetCube) (Math|Vector|MakeVector (.x _location) (.y _location) (+ (.z _location) _newtrack_0)) false false))))

(event EventBeginPlay
  (Variables|Default|SetLocation (Transformation|GetWorldLocation (Variables|Default|GetCube))))

(fn ConstructionScript)